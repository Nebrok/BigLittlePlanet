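; BP_Homeplanet is the home planet Blueprint that drives the game's day cycle and recurring running cost.
; Tick accumulates delta time in a timer, which resets to zero once it passes two seconds.
; Each reset advances CurrentDay on the HomeplanetManager and subtracts its MoneyCostPerDay from TotalMoney, with no check on the remaining balance.
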(event EventTick
  (params (DeltaSeconds :type Float%20%28single-precision%29))
  (bind _returnvalue (Subsystems|GetHomeplanetManager))
  (bind _output_get (Variables|Default|SetTimer (+ DeltaSeconds (Variables|Default|GetTimer))))
  (Math|Float|CompareFloat _output_get 2.0
    (:>
      (Variables|Default|SetTimer 0.0)
      (Math|Integer|IncrementInt (Variables|/Script/BigLittlePlanet.HomeplanetManager|GetcurrentDay _returnvalue)
        (:%20%20
          (Variables|/Script/BigLittlePlanet.HomeplanetManager|SettotalMoney _returnvalue (- (Variables|/Script/BigLittlePlanet.HomeplanetManager|GettotalMoney _returnvalue) (Variables|/Script/BigLittlePlanet.HomeplanetManager|GetmoneyCostPerDay _returnvalue))))))))

(fn ConstructionScript)