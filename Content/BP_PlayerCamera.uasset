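; Player camera Blueprint that sets up Enhanced Input and moves the camera while the mouse is held.
; BeginPlay stores its Camera component as GamePlayCamera and adds the input mapping context for the first player.
; Ongoing mouse-hold input calls MoveCamera, which is defined outside this graph.
; A completed click shorter than a brief threshold only prints a debug message, and Tick is empty.
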(event Input|EnhancedActionEvents|EnhancedInputActionIA_MouseClick
  (params (ActionValue :type Boolean) (ElapsedSeconds :type Float%20%28double-precision%29) (TriggeredSeconds :type Float%20%28double-precision%29) (InputAction :type Input%20Action%20Object%20Reference :default "/Game/Inputs/IA_MouseClick.IA_MouseClick"))
  (:Completed
    (Math|Float|CompareFloat ElapsedSeconds 0.1
      (:<
        (Development|PrintString "Click")))))

(event Input|EnhancedActionEvents|EnhancedInputActionIA_MouseHold
  (params (ActionValue :type Boolean) (ElapsedSeconds :type Float%20%28double-precision%29) (TriggeredSeconds :type Float%20%28double-precision%29) (InputAction :type Input%20Action%20Object%20Reference :default "/Game/Inputs/IA_MouseHold.IA_MouseHold"))
  (:Ongoing
    (Class|PlayerCamera|MoveCamera (stale EventTick DeltaSeconds))))

(event EventBeginPlay
  (Variables|Default|SetgamePlayCamera (Variables|Default|GetCamera))
  (Input|AddMappingContext (PlayerController|LocalPlayerSubsystems|GetEnhancedInputLocalPlayerSubsystem (Game|GetPlayerController 0)) "/Game/Inputs/Mapping.Mapping" 0 "(bIgnoreAllPressedKeysUntilRelease=True,bForceImmediately=False,bNotifyUserSettings=False)"))

(event EventTick
  (params (DeltaSeconds :type Float%20%28single-precision%29)))

(fn ConstructionScript)